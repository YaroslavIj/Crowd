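; Game mode for a timed crowd-hunting game: the player wins by killing every AI character before difficulty-scaled time runs out.
; BeginPlay applies saved difficulty and optimization, sets up animation sharing and budgeting, and spawns a non-overlapping crowd near a random tagged TargetPoint.
; The crowd shares one move target, wandering to random navigable points or running away from the player when found.
; Kills and the countdown update the HUD; either ending shows the end-game widget and pauses.
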(event `SetTimerToAIStopRunFromCharacter`)

(event `StopAIRunFromCharacter`
  (for _ (`self.AICharacters`)
    (`self.Player Found` (`GameplayStatics.GetPlayerPawn` 0))))

(event `AICharacterArrivedToTarget`
  (params (Character :type "/Game/BP/BP_AICharacter Object Reference"))
  (if (not (`KismetSystemLibrary.K2_IsTimerActiveHandle` (`self.TimerToFindNewAITargetLocation`)))
    (bind _returnvalue (`KismetSystemLibrary.K2_SetTimerDelegate` (delegate `CustomEvent`) 5.0))
    (set `self.TimerToFindNewAITargetLocation` _returnvalue)))

(event `CustomEvent`
  (`self.FindRandomPointToAIMove`)
  (`self.Set AICharacters Movement State` false))

(event `self.ReceiveBeginPlay`
  (bind _returnvalue (`KismetSystemLibrary.K2_SetTimerDelegate` (delegate `DecreaseGameTime`) 1.0 true))
  (set `self.GameTimer` _returnvalue)
  (bind _asbp_game_instance (cast `/Game/BP/BP_GameInstance` (`GameplayStatics.GetGameInstance`)))
  (bind (_skin _difficult _boptimize) (`/Game/BP/BP_GameInstance.GetSavedParameters` _asbp_game_instance))
  (bind _output_get (set `self.bOptimize` _boptimize))
  (`AnimationBudgetBlueprintLibrary.EnableAnimationBudget` _output_get)
  (set `self.AIMaxCharactersCount` (select `int` _difficult :`0` 10 :`1` 30 :`2` 50 :`3` 80))
  (bind _returnvalue_2 (select `int` _difficult :`0` 120.0 :`1` 240.0 :`2` 270.0 :`3` 300.0))
  (set `self.MaxGameTime` _returnvalue_2)
  (set `self.GameTime` _returnvalue_2)
  (`AnimationSharingManager.CreateAnimationSharingManager` (select `int` _difficult :`0` "/Game/Animation/AIAnimSharingSetup_10.AIAnimSharingSetup_10" :`1` "/Game/Animation/AIAnimSharingSetup_30.AIAnimSharingSetup_30" :`2` "/Game/Animation/AIAnimSharingSetup_50.AIAnimSharingSetup_50" :`3` "/Game/Animation/AIAnimSharingSetup_80.AIAnimSharingSetup_80" :!type "AnimationSharingSetup Object Reference"))
  (`self.SpawnAICharacters` (`self.AIMaxCharactersCount`)))

(event `DecreaseGameTime`
  (bind _output_get (set `self.GameTime` (- (`self.GameTime`) 1.0)))
  (if (<= _output_get 0.0)
    (set `self.GameTime` 0.0)
    (`self.TimeOver`))
  (bind _asbp_player_controller (cast `/Game/BP/BP_PlayerController` (`GameplayStatics.GetPlayerController` 0)))
  (`/Game/BP/Widgets/BPW_Main.SetGameTime` (`/Game/BP/BP_PlayerController.MainWidget` _asbp_player_controller) (`KismetMathLibrary.FTrunc` (`self.GameTime`))))

(event `OnPlayerFound`
  (`KismetSystemLibrary.K2_SetTimerDelegate` (delegate `SetCanFindPlayer`) 0.2))

(event `OnAIKilled`
  (params (Character :type "/Game/BP/BP_AICharacter Object Reference"))
  (bind _aicharacters (`self.AICharacters`))
  (bind _returnvalue (`KismetArrayLibrary.Array_RemoveItem` _aicharacters Character))
  (`self.K2_DestroyActor` Character)
  (if _returnvalue
    (if (<= (`KismetArrayLibrary.Array_Length` _aicharacters) 0)
      (bind (_kills _remainingaicharacters _remaininggametime _wastedtime) (`self.GetGameInfo`))
      (bind _returnvalue_2 (`|CreateWidget` "/Game/BP/Widgets/BPW_EndGame.BPW_EndGame_C" null _kills (`KismetMathLibrary.FTrunc` _wastedtime) true))
      (`UserWidget.AddToViewport` _returnvalue_2 0)
      (set `PlayerController.bShowMouseCursor` true (`GameplayStatics.GetPlayerController` 0))
      (`self.EndGame`))
    (bind _asbp_player_controller (cast `/Game/BP/BP_PlayerController` (`GameplayStatics.GetPlayerController` 0)))
    (`/Game/BP/Widgets/BPW_Main.SetEnemies` (`/Game/BP/BP_PlayerController.MainWidget` _asbp_player_controller) (`KismetArrayLibrary.Array_Length` (`self.AICharacters`)))))

(event `SetCanFindPlayer`
  (set `self.bCanFindPlayer` true))

(event `self.ReceiveTick`
  (params (DeltaSeconds :type "Float (single-precision)")))

(event `TimeOver`
  (bind (_kills _remainingaicharacters _remaininggametime _wastedtime) (`self.GetGameInfo`))
  (bind _returnvalue (`|CreateWidget` "/Game/BP/Widgets/BPW_EndGame.BPW_EndGame_C" null _kills (`KismetMathLibrary.FTrunc` _wastedtime)))
  (`UserWidget.AddToViewport` _returnvalue 0)
  (set `PlayerController.bShowMouseCursor` true (`GameplayStatics.GetPlayerController` 0))
  (`self.EndGame`))

(event `EndGame`
  (bind _asbp_player_controller (cast `/Game/BP/BP_PlayerController` (`GameplayStatics.GetPlayerController` 0)))
  (`Widget.RemoveFromParent` (`/Game/BP/BP_PlayerController.MainWidget` _asbp_player_controller))
  (`KismetSystemLibrary.K2_ClearAndInvalidateTimerHandle` (`self.GameTimer`))
  (`GameplayStatics.SetGamePaused` true))

(fn `FindRandomPointToAIMove`
  (locals (NewLocation :type "Vector Structure") (bIsSuccess :type Boolean))
  (while (not (`local.bIsSuccess`))
    (bind _output_get (set `local.NewLocation` (`NavigationSystemV1.K2_GetRandomReachablePointInRadius` (`self.CurrentAICharactersTargetLocation`) 6000.0 null null)))
    (if (> (`KismetMathLibrary.VSize` (- _output_get (`self.CurrentAICharactersTargetLocation`))) 3000.0)
      (set `self.CurrentAICharactersTargetLocation` (`local.NewLocation`))
      (`self.UpdateAITargetLocation`)
      (set `local.bIsSuccess` true))))

(fn `GetGameInfo`
  (returns (Kills :type Integer) (RemainingAICharacters :type Integer) (RemainingGameTime :type "Float (double-precision)") (WastedTime :type "Float (double-precision)"))
  (bind _gametime (`self.GameTime`))
  (bind _returnvalue (`KismetArrayLibrary.Array_Length` (`self.AICharacters`)))
  (return (- (`self.AIMaxCharactersCount`) _returnvalue) _returnvalue _gametime (- (`self.MaxGameTime`) _gametime)))

(fn `Player Found`
  (params (FoundedActor :type "Actor Object Reference"))
  (locals (FarthestCharacterLocation :type "Vector Structure") (PlayerCharacterLocation :type "Vector Structure" :default (0.0 0.0 0.0)) (BiggestXLocation :type "Float (double-precision)") (SmallestXLocation :type "Float (double-precision)") (BiggestYLocation :type "Float (double-precision)") (SmallestYLocation :type "Float (double-precision)") (MiddleCrowdLocation :type "Vector Structure"))
  (bind (_playercharacterlocation_x _playercharacterlocation_y) (`KismetMathLibrary.BreakVector` (`local.PlayerCharacterLocation`)))
  (if (`self.bCanFindPlayer`)
    (if (== (`GameplayStatics.GetObjectClass` FoundedActor) "/Game/BP/BP_Character.BP_Character_C")
      (set `self.bCanFindPlayer` false)
      (`self.Set AICharacters Movement State` true)
      (`KismetSystemLibrary.K2_ClearAndInvalidateTimerHandle` (`self.TimerToFindNewAITargetLocation`))
      (set `local.PlayerCharacterLocation` (`self.K2_GetActorLocation` FoundedActor))
      (for (_array_element _array_index) (`self.AICharacters`)
        (if (== _array_index 0)
          (bind (_returnvalue_x _returnvalue_y) (`KismetMathLibrary.BreakVector` (`self.K2_GetActorLocation` _array_element)))
          (set `local.BiggestXLocation` _returnvalue_x)
          (set `local.SmallestXLocation` _returnvalue_x)
          (set `local.BiggestYLocation` _returnvalue_y)
          (set `local.SmallestYLocation` _returnvalue_y)
          (else
            (`|ExecutionSequence`
              (:`then_0`
                (if (> _returnvalue_x (`local.BiggestXLocation`))
                  (set `local.BiggestXLocation` _returnvalue_x)
                  (elif (< _returnvalue_x (`local.SmallestXLocation`))
                    (set `local.SmallestXLocation` _returnvalue_x))))
              (:`then_1`
                (if (> _returnvalue_y (`local.BiggestYLocation`))
                  (set `local.BiggestYLocation` _returnvalue_y)
                  (elif (< _returnvalue_y (`local.SmallestYLocation`))
                    (set `local.SmallestYLocation` _returnvalue_y))))))))
      (bind _output_get (set `local.MiddleCrowdLocation` (`KismetMathLibrary.MakeVector` (/ (+ (`local.BiggestXLocation`) (`local.SmallestXLocation`)) 2.0) (/ (+ (`local.BiggestYLocation`) (`local.SmallestYLocation`)) 2.0) 1000.0)))
      (`KismetSystemLibrary.DrawDebugSphere` (`KismetMathLibrary.MakeVector` (.x _output_get) (.y _output_get)) 30.0 12 (struct :`R` 1.0 :`G` 1.0 :`B` 1.0 :`A` 1.0) 2.0)
      (bind _returnvalue (+ _output_get (* (`KismetMathLibrary.Normal` (- _output_get (`KismetMathLibrary.MakeVector` _playercharacterlocation_x _playercharacterlocation_y 1000.0))) 5000.0)))
      (bind _outhit (`KismetSystemLibrary.LineTraceSingle` :`Start` _returnvalue :`End` (`KismetMathLibrary.MakeVector` (.x _returnvalue) (.y _returnvalue) -1000.0) :`TraceChannel` "TraceTypeQuery1" :`DrawDebugType` "ForDuration" :`DrawTime` 0.2))
      (bind (_bblockinghit _binitialoverlap _time _distance _location _impactpoint) (`GameplayStatics.BreakHitResult` _outhit))
      (if (`.ReturnValue` (`NavigationSystemV1.K2_ProjectPointToNavigation` _impactpoint))
        (set `self.CurrentAICharactersTargetLocation` _impactpoint)
        (`self.UpdateAITargetLocation`)
        (`self.OnPlayerFound`)
        (else
          (`self.FindRandomPointToAIMove`)
          (`self.OnPlayerFound`))))))

(fn `Set AICharacters Movement State`
  (params (bIsRun :type Boolean))
  (for _array_element (`self.AICharacters`)
    (`/Game/BP/BP_AICharacter.SetMovementState` _array_element bIsRun)))

(fn `SpawnAICharacters`
  (params (Count :type Integer))
  (locals (UnitSquare :type "Float (double-precision)" :default 11775.0) (bIsSuccess :type Boolean :default false) (SpawnLocation :type "Vector Structure") (SpawnScale :type "Float (double-precision)") (TargetPoints :type "Array of TargetPoint Object Reference") (TargetPointLocation :type "Vector Structure" :default (0.0 0.0 0.0)))
  (bind _returnvalue (`KismetMathLibrary.RandomFloatInRange` 0.8 1.2))
  (bind _targetpointlocation (`local.TargetPointLocation`))
  (bind (_distance _returnvalue_2) (`GameplayStatics.FindNearestActor` (`local.SpawnLocation`) (`self.AICharacters`)))
  (bind _returnvalue_x (`KismetMathLibrary.BreakVector` (`self.GetActorScale3D` _returnvalue_2)))
  (bind _randomlocation (`NavigationSystemV1.K2_GetRandomReachablePointInRadius` _targetpointlocation (`KismetMathLibrary.Sqrt` (/ (* Count (`local.UnitSquare`)) 3.14)) null null))
  (bind _outactors (`GameplayStatics.GetAllActorsOfClass` "/Script/Engine.TargetPoint"))
  (for _array_element _outactors
    (if (== (`|GetArrayItem` (`Actor.Tags` _array_element)) "AISpawnPoint")
      (`KismetArrayLibrary.Array_Add` (`local.TargetPoints`) _array_element)))
  (set `local.TargetPointLocation` (`self.K2_GetActorLocation` (`KismetArrayLibrary.Array_Random` (`local.TargetPoints`))))
  (for _index (range Count)
    (set `local.bIsSuccess` false)
    (set `local.SpawnScale` (`KismetMathLibrary.RandomFloatInRange` 0.8 1.2))
    (if (!= _index 0)
      (for _ (range 101)
        (set `local.SpawnLocation` (`KismetMathLibrary.MakeVector` (.x _randomlocation) (.y _randomlocation) (.z _targetpointlocation)))
        (if (> _distance (+ (`KismetMathLibrary.MapRangeClamped` _returnvalue_x 0.8 1.2 28.0 42.0) (`KismetMathLibrary.MapRangeClamped` (`local.SpawnScale`) 0.8 1.2 28.0 42.0)))
          (set `local.bIsSuccess` true)
          (break)))
      (if (`local.bIsSuccess`)
        (bind _returnvalue_3 (`|SpawnActorFromClass` "/Game/BP/BP_AICharacter.BP_AICharacter_C" (`KismetMathLibrary.MakeTransform` (`local.SpawnLocation`) (struct) (`KismetMathLibrary.MakeVector` _returnvalue _returnvalue _returnvalue)) "AlwaysSpawn" "MultiplyWithRoot" null null :!label _label))
        (`KismetArrayLibrary.Array_Add` (`self.AICharacters`) _returnvalue_3)
        (`/Game/BP/BP_AICharacter.SetMovementState` _returnvalue_3 false)
        (else
          (`/Engine/EditorBlueprintResources/StandardMacros.DecrementInt` (`self.AIMaxCharactersCount`)
            (:`  `
              (`KismetSystemLibrary.PrintString` "Character Hasn't Found Greate Place to Spawn" true true (struct :`G` 0.66 :`B` 1.0 :`A` 1.0) 10.0)))))
      (else
        (set `local.SpawnLocation` _targetpointlocation)
        (goto _label))))
  (set `self.CurrentAICharactersTargetLocation` _targetpointlocation)
  (`self.UpdateAITargetLocation`))

(fn `UpdateAITargetLocation`
  (for _array_element (`self.AICharacters`)
    (set `/Game/BP/BP_AICharacter.MoveTargetLocation` (`self.CurrentAICharactersTargetLocation`) _array_element)))

(fn `UserConstructionScript`)