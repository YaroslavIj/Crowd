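; Player controller for the menu, which puts the BPW_Menu widget on screen and shows the mouse cursor on BeginPlay.
; It then reads the saved parameters from BP_GameInstance and checks whether the saved Skin is valid.
; A second sequence branch repeats that check, but neither check leads to any action, and Tick is unused.
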(event `self.ReceiveBeginPlay`
  (`|ExecutionSequence`
    (:`then_0`
      (bind _returnvalue (`|CreateWidget` "/Game/BP/Widgets/BPW_Menu.BPW_Menu_C" null null))
      (`UserWidget.AddToViewport` _returnvalue 0)
      (set `self.bShowMouseCursor` true)
      (bind _asbp_game_instance (cast `/Game/BP/BP_GameInstance` (`GameplayStatics.GetGameInstance`)))
      (bind _skin (`/Game/BP/BP_GameInstance.GetSavedParameters` _asbp_game_instance))
      (`/Engine/EditorBlueprintResources/StandardMacros.IsValid` _skin))
    (:`then_1`
      (bind _asbp_game_instance_2 (cast `/Game/BP/BP_GameInstance` (`GameplayStatics.GetGameInstance`)))
      (bind _skin_2 (`/Game/BP/BP_GameInstance.GetSavedParameters` _asbp_game_instance_2))
      (`/Engine/EditorBlueprintResources/StandardMacros.IsValid` _skin_2))))

(fn `UserConstructionScript`)