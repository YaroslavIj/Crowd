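; Player controller that creates the main HUD, seeding it with the game mode's maximum AI count, and handles the pause menu.
; Escape opens a pause widget with kills, time and remaining enemies from the game mode, pauses the game and its timer, and hides the HUD.
; Debug keys enable Animation Budget Allocator stats and toggle its budget between tiny and generous values to compare performance.
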(event `self.ReceiveBeginPlay`
  (bind _returnvalue (`|CreateWidget` "/Game/BP/Widgets/BPW_Main.BPW_Main_C"))
  (`UserWidget.AddToViewport` _returnvalue 0)
  (set `self.MainWidget` _returnvalue)
  (bind _asbp_game_mode (cast `/Game/BP/BP_GameMode` (`GameplayStatics.GetGameMode`)))
  (`/Game/BP/Widgets/BPW_Main.SetEnemies` _returnvalue (`/Game/BP/BP_GameMode.AIMaxCharactersCount` _asbp_game_mode)))

(event `Key|One`
  (params (Key :type "Key Structure"))
  (:`Pressed`
    (`KismetSystemLibrary.ExecuteConsoleCommand` "a.Budget.Enabled 1" null)
    (`KismetSystemLibrary.ExecuteConsoleCommand` "a.Budget.Debug.Enabled 1" null)
    (`KismetSystemLibrary.ExecuteConsoleCommand` "Stat AnimationBudgetAllocator" null)))

(event `Key|Two`
  (params (Key :type "Key Structure"))
  (:`Pressed`
    (`/Engine/EditorBlueprintResources/StandardMacros.FlipFlop`
      (:`A`
        (`AnimationBudgetBlueprintLibrary.SetAnimationBudgetParameters` (make `AnimationBudgetAllocatorParameters` 0.001)))
      (:`B`
        (`AnimationBudgetBlueprintLibrary.SetAnimationBudgetParameters` (make `AnimationBudgetAllocatorParameters` 30.0))))))

(event `self.ReceiveEndPlay`
  (params (EndPlayReason :type "EEndPlayReason Enum" :default "Destroyed")))

(event `Key|Escape`
  (params (Key :type "Key Structure"))
  (:`Pressed`
    (bind _asbp_game_mode (cast `/Game/BP/BP_GameMode` (`GameplayStatics.GetGameMode`)))
    (bind (_kills _remainingaicharacters _remaininggametime) (`/Game/BP/BP_GameMode.GetGameInfo` _asbp_game_mode))
    (bind _returnvalue (`|CreateWidget` "/Game/BP/Widgets/BPW_Pause.BPW_Pause_C" null _kills (`KismetMathLibrary.FTrunc` _remaininggametime) _remainingaicharacters))
    (`UserWidget.AddToViewport` _returnvalue 0)
    (set `self.bShowMouseCursor` true)
    (`KismetSystemLibrary.K2_PauseTimerHandle` (`/Game/BP/BP_GameMode.GameTimer` _asbp_game_mode))
    (`GameplayStatics.SetGamePaused` true)
    (`Widget.SetVisibility` (`self.MainWidget`) "Hidden")))

(fn `UserConstructionScript`)