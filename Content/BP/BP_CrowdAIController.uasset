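; BP_CrowdAIController is the AI controller for crowd characters that reports perceived actors to the game mode.
; On possess, it caches the pawn as a BP_AICharacter.
; When AI perception updates, it passes the actor to BP_GameMode's PlayerFound if that character is valid and has health above zero.
; The handler does not filter by actor type or by whether the target was gained or lost.
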(event `self.ReceivePossess`
  (params (PossessedPawn :type "Pawn Object Reference"))
  (bind _asbp_aicharacter (cast `/Game/BP/BP_AICharacter` PossessedPawn))
  (set `self.AICharacter` _asbp_aicharacter))

(event `self.AIPerception.OnTargetPerceptionUpdated`
  (params (Actor :type "Actor Object Reference") (Stimulus :type "AIStimulus Structure"))
  (bind _aicharacter (`self.AICharacter`))
  (`/Engine/EditorBlueprintResources/StandardMacros.IsValid` _aicharacter
    (:`Is Valid`
      (if (> (`/Game/BP/BP_AICharacter.Health` _aicharacter) 0.0)
        (bind _asbp_game_mode (cast `/Game/BP/BP_GameMode` (`GameplayStatics.GetGameMode`)))
        (`/Game/BP/BP_GameMode.Player Found` _asbp_game_mode Actor)))))

(fn `UserConstructionScript`)